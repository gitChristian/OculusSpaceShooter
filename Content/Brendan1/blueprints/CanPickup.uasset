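; Configurable pickup item that the first-person player can collect into the inventory and later use to gain health, energy and rage.
; The construction script fills its inventory struct and sets the mesh from variables.
; A trigger shows a prompt widget and gates the pickup event bound through the character.
; Pickup hides the actor and disables collision, keeping it referenced in the HUD inventory until UseAction applies the stats and destroys it.
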(event `self.ReceiveBeginPlay`
  (bind _item_info (`self.Item Info`))
  (bind (_item _itemimage _pickuptext) (break `/Game/FirstPersonBP/Brendan1/blueprints/InventoryStruct` _item_info))
  ;[1 1 1] Event Begin Play
  (bind _returnvalue (`|CreateWidget` "/Game/FirstPersonBP/UMG/UMG/PickupText.PickupText_C"))
  (set `self.PickupText Widget` _returnvalue)
  (set `/Game/FirstPersonBP/UMG/UMG/PickupText.PickupActor` _item _returnvalue)
  (set `/Game/FirstPersonBP/UMG/UMG/PickupText.PickupText` _pickuptext _returnvalue)
  (setmembers `/Game/FirstPersonBP/Brendan1/blueprints/InventoryStruct` :`StructRef` _item_info :`Item` self)
  (bind _asfirst_person_character (cast `/Game/FirstPersonBP/Brendan1/blueprints/FirstPersonCharacter` (`GameplayStatics.GetPlayerCharacter` 0)))
  (set `self.My Character` _asfirst_person_character)
  (add `/Game/FirstPersonBP/Brendan1/blueprints/FirstPersonCharacter.PickupItem` _asfirst_person_character (delegate `PickupItem_Event_0`)))

(event `self.Trigger.OnComponentBeginOverlap`
  (params (OtherActor :type "Actor Object Reference") (OtherComp :type "PrimitiveComponent Object Reference") (OtherBodyIndex :type Integer) (bFromSweep :type Boolean) (SweepResult :type "EngineTypes.HitResult Structure (by ref)"))
  ;[1 1 1] Triggers
  (cast `/Game/FirstPersonBP/Brendan1/blueprints/FirstPersonCharacter` OtherActor)
  (`UserWidget.AddToViewport` (`self.PickupText Widget`) 0)
  (set `self.IsInRange` true))

(event `PickupItem_Event_0`
  (bind _game_hudwidget (`/Game/FirstPersonBP/Brendan1/blueprints/FirstPersonCharacter.Game HudWidget` (`self.My Character`)))
  ;[1 1 1] Pickup and add item to inventory
  (if (and (`self.GetActorEnableCollision`) (`self.IsInRange`))
    (`KismetArrayLibrary.Array_Add` (`/Game/FirstPersonBP/UMG/UMG/GameHud.Inventory` _game_hudwidget) (`self.Item Info`))
    (`Widget.RemoveFromParent` (`self.PickupText Widget`))
    (`self.SetActorHiddenInGame` true)
    (`self.SetActorEnableCollision` false)
    (`/Game/FirstPersonBP/UMG/UMG/GameHud.Refresh Inventory` _game_hudwidget)))

(event `self.Trigger.OnComponentEndOverlap`
  (params (OtherActor :type "Actor Object Reference") (OtherComp :type "PrimitiveComponent Object Reference") (OtherBodyIndex :type Integer))
  ;[1 1 1] Triggers
  (cast `/Game/FirstPersonBP/Brendan1/blueprints/FirstPersonCharacter` OtherActor)
  (`Widget.RemoveFromParent` (`self.PickupText Widget`))
  (set `self.IsInRange` false))

(event `self.Use Action`
  (bind _my_character (`self.My Character`))
  ;[1 1 1] Item was used
  (set `/Game/FirstPersonBP/Brendan1/blueprints/FirstPersonCharacter.Health` (+ (`/Game/FirstPersonBP/Brendan1/blueprints/FirstPersonCharacter.Health` _my_character) (`self.AddHealth`)) _my_character)
  (set `/Game/FirstPersonBP/Brendan1/blueprints/FirstPersonCharacter.Energy` (+ (`/Game/FirstPersonBP/Brendan1/blueprints/FirstPersonCharacter.Energy` _my_character) (`self.AddEnergy`)) _my_character)
  (set `/Game/FirstPersonBP/Brendan1/blueprints/FirstPersonCharacter.Rage` (+ (`/Game/FirstPersonBP/Brendan1/blueprints/FirstPersonCharacter.Rage` _my_character) (`self.AddRage`)) _my_character)
  (`self.K2_DestroyActor`))

(fn `UserConstructionScript`
  (setmembers `/Game/FirstPersonBP/Brendan1/blueprints/InventoryStruct` :`StructRef` (`self.Item Info`) :`Item` self :`ItemImage` (`self.InventoryImage`) :`PickupText` (`self.PickupText`) :`ActionText` (`self.ActionText`))
  (`StaticMeshComponent.SetStaticMesh` (`self.Can`) (`self.CustomMesh`)))