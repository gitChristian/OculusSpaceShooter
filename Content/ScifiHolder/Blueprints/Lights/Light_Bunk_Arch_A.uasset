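; Bunk arch light fixture Blueprint that drives a mesh's emissive material and its two lights from shared colour and multiplier variables.
; The construction script creates a dynamic material instance on the mesh and sets its emissive parameters.
; It also colours LightRadius and LightSpotB and scales their intensity from the multiplier, with the spot at twice the factor.
; Tick repeats all of this every frame, including the dynamic material instance creation call.
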(event `self.ReceiveTick`
  (params (DeltaSeconds :type "Float (single-precision)"))
  (bind _light_spot_b (`self.Light_Spot_B`))
  (bind _emissive_colour (`self.Emissive Colour`))
  (bind _emissive_multiply (`self.Emissive Multiply`))
  (bind _light_radius (`self.Light_Radius`))
  (bind _returnvalue (`PrimitiveComponent.CreateDynamicMaterialInstance` (`self.SM_Light_Bunk_Arch_A`) 0 null))
  (`MaterialInstanceDynamic.SetScalarParameterValue` _returnvalue "EmissiveMultiply" _emissive_multiply)
  (`MaterialInstanceDynamic.SetVectorParameterValue` _returnvalue "EmissiveCol" _emissive_colour)
  (`LightComponent.SetIntensity` _light_radius (* _emissive_multiply 1000.0))
  (`LightComponent.SetLightColor` _light_radius _emissive_colour)
  (`LightComponent.SetIntensity` _light_spot_b (* _emissive_multiply 2000.0))
  (`LightComponent.SetLightColor` _light_spot_b _emissive_colour))

(fn `UserConstructionScript`
  (bind _light_spot_b (`self.Light_Spot_B`))
  (bind _emissive_colour (`self.Emissive Colour`))
  (bind _emissive_multiply (`self.Emissive Multiply`))
  (bind _light_radius (`self.Light_Radius`))
  (bind _returnvalue (`PrimitiveComponent.CreateDynamicMaterialInstance` (`self.SM_Light_Bunk_Arch_A`) 0 null))
  (`MaterialInstanceDynamic.SetScalarParameterValue` _returnvalue "EmissiveMultiply" _emissive_multiply)
  (`MaterialInstanceDynamic.SetVectorParameterValue` _returnvalue "EmissiveCol" _emissive_colour)
  (`LightComponent.SetIntensity` _light_radius (* _emissive_multiply 1000.0))
  (`LightComponent.SetIntensity` _light_spot_b (* _emissive_multiply 2000.0))
  (`LightComponent.SetLightColor` _light_spot_b _emissive_colour)
  (`LightComponent.SetLightColor` _light_radius _emissive_colour))